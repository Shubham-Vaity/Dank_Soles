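; BP_enemy is an enemy character Blueprint that supplies attack and idle actions, each returning a duration.
; Attack uses chained coin flips to play one of four punch montages, weighted toward the first, and returns its length.
; IdleShit always plays the stand-to-roll montage because its random check always passes, leaving the jump fallback unreachable.
; The event graph is empty, and nothing in this file calls either function.
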(fn `Attack`
  (returns (`Duration ` :type "Float (double-precision)"))
  (bind _returnvalue (`KismetMathLibrary.RandomBool`))
  (if _returnvalue
    (bind _returnvalue_2 (`self.PlayAnimMontage` "/Game/Dank/models/Enemys/zombie/Montages/Cross_Punch_Montage.Cross_Punch_Montage"))
    (return _returnvalue_2)
    (elif _returnvalue
      (bind _returnvalue_3 (`self.PlayAnimMontage` "/Game/Dank/models/Enemys/zombie/Montages/Hook_Punch_Montage_attack1.Hook_Punch_Montage_attack1"))
      (return _returnvalue_3)
      (elif _returnvalue
        (bind _returnvalue_4 (`self.PlayAnimMontage` "/Game/Dank/models/Enemys/zombie/Montages/MTG_Punch.MTG_Punch"))
        (return _returnvalue_4)
        (else
          (bind _returnvalue_5 (`self.PlayAnimMontage` "/Game/Dank/models/Enemys/zombie/Montages/Punching__1__Montage.Punching__1__Montage"))
          (return _returnvalue_5))))))

(fn `IdleShit`
  (returns (delay :type "Float (double-precision)"))
  (bind _returnvalue (`KismetMathLibrary.RandomInteger` 100))
  (if (< _returnvalue 100)
    (bind _returnvalue_2 (`self.PlayAnimMontage` "/Game/Dank/models/Enemys/zombie/Montages/Stand_To_Roll_Montage.Stand_To_Roll_Montage"))
    (return _returnvalue_2)
    (elif (> _returnvalue 100)
      (`self.Jump`)
      (return 0.5)
      (else
        (return 0.0)))))

(fn `UserConstructionScript`)