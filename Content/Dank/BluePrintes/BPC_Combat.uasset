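; Combat component for the third-person player character, handling target lock-on and a two-handed sword combo.
; Lock input sphere-traces from the camera for a pawn, attaches a dot marker and aims control rotation at it each tick.
; Attack input plays one montage, stopping at notifies unless another press buffered the combo.
; A looping timer runs debug-drawn sword sphere traces between begin/end events, but applies no damage yet.
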(event `self.ReceiveTick`
  (params (DeltaSeconds :type "Float (single-precision)"))
  (bind _playerreff (`self.PlayerReff`))
  (bind (_returnvalue_roll _returnvalue_pitch _returnvalue_yaw) (`KismetMathLibrary.BreakRotator` (`KismetMathLibrary.FindLookAtRotation` (`Actor.K2_GetActorLocation` _playerreff) (`Actor.K2_GetActorLocation` (`self.TargetLocakActor`)))))
  ; tick
  (`self.TargetLocakActor`
    (:`then`
      (`Controller.SetControlRotation` (`Pawn.GetController` _playerreff) (`KismetMathLibrary.MakeRotator` _returnvalue_roll (- _returnvalue_pitch 26.9) _returnvalue_yaw)))
    (:`else`)))

(event `self.ReceiveBeginPlay`
  ; Reff
  (bind _asbp_third_person_character (cast `/Game/ThirdPerson/Blueprints/BP_ThirdPersonCharacter` (`self.GetOwner`)))
  (set `self.PlayerReff` _asbp_third_person_character))

(event `EnhancedInput|/Game/ThirdPerson/Input/Actions/IA_Lock`
  (params (ActionValue :type Boolean) (ElapsedSeconds :type "Float (double-precision)") (TriggeredSeconds :type "Float (double-precision)") (InputAction :type "InputAction Object Reference" :default "/Game/ThirdPerson/Input/Actions/IA_Lock.IA_Lock"))
  (bind (_returnvalue_location _returnvalue_rotation) (`KismetMathLibrary.BreakTransform` (`Actor.GetTransform` (`self.TargetLocakActor`))))
  (bind _transformcomponent (`PlayerCameraManager.TransformComponent` (`GameplayStatics.GetPlayerCameraManager` 0)))
  (bind _charactermovement (`Character.CharacterMovement` (`self.PlayerReff`)))
  (bind _charactermovement_2 (`Character.CharacterMovement` (`self.PlayerReff`)))
  (bind (_returnvalue_x _returnvalue_y _returnvalue_z) (`KismetMathLibrary.BreakVector` (`SceneComponent.K2_GetComponentLocation` _transformcomponent)))
  (bind _returnvalue (`KismetMathLibrary.MakeVector` _returnvalue_x _returnvalue_y (+ _returnvalue_z 69.0)))
  ; Lock/Unlock
  (:`Started`
    (`self.TargetLocakActor`
      (:`then`
        (set `self.TargetLocakActor` null)
        (set `CharacterMovementComponent.bOrientRotationToMovement` true _charactermovement)
        (set `CharacterMovementComponent.bUseControllerDesiredRotation` false _charactermovement)
        (`Actor.K2_DestroyActor` (`self.LOCK Dot`)))
      (:`else`
        (bind (_outhit _returnvalue_2) (`KismetSystemLibrary.SphereTraceSingleForObjects` _returnvalue (+ _returnvalue (* (`KismetMathLibrary.GetForwardVector` (`SceneComponent.K2_GetComponentRotation` _transformcomponent)) 1696.0)) 169.0 (`|MakeArray` "ObjectTypeQuery3" :!type "EObjectTypeQuery Enum")))
        (if _returnvalue_2
          (set `self.TargetLocakActor` (`.HitActor` (`GameplayStatics.BreakHitResult` _outhit)))
          (set `CharacterMovementComponent.bOrientRotationToMovement` false _charactermovement_2)
          (set `CharacterMovementComponent.bUseControllerDesiredRotation` true _charactermovement_2)
          (bind _returnvalue_3 (`|SpawnActorFromClass` "/Game/Dank/BluePrintes/BP_target_dot.BP_target_dot_C" (`KismetMathLibrary.MakeTransform` _returnvalue_location _returnvalue_rotation) "AlwaysSpawn" "MultiplyWithRoot" null null))
          (bind _output_get (set `self.LOCK Dot` _returnvalue_3))
          (`Actor.K2_AttachToActor` _output_get (`self.TargetLocakActor`) "None" "SnapToTarget" "SnapToTarget" "SnapToTarget" true))))))

(event `EndDamage Trace`
  ; sword traces
  (if (`KismetSystemLibrary.K2_IsValidTimerHandle` (stale `Begin DamageLineTrace` _returnvalue))
    (`KismetSystemLibrary.K2_ClearAndInvalidateTimerHandle` (stale `Begin DamageLineTrace` _returnvalue))))

(event `Begin DamageLineTrace`
  ; sword traces
  (bind _returnvalue (`KismetSystemLibrary.K2_SetTimerDelegate` (delegate `DamageTrace`) 0.01 true)))

(event `EnhancedInput|/Game/ThirdPerson/Input/Actions/IA_attack`
  (params (ActionValue :type Boolean) (ElapsedSeconds :type "Float (double-precision)") (TriggeredSeconds :type "Float (double-precision)") (InputAction :type "InputAction Object Reference" :default "/Game/ThirdPerson/Input/Actions/IA_attack.IA_attack"))
  (bind _mesh (`Character.Mesh` (`self.PlayerReff`)))
  ; Attack ANimation
  (:`Started`
    (if (not (`self.isattacking`))
      (set `self.isattacking` true)
      (`SceneComponent.K2_SetRelativeRotation` _mesh (`KismetMathLibrary.MakeRotator` 0.0) false false)
      (`|PlayMontage` _mesh "/Game/Dank/Player1/animation/YTanimations/Animations/montag/Two_Hand_Sword_Combo_Montage.Two_Hand_Sword_Combo_Montage"
        (:`OnCompleted`
          (set `self.isattacking` false :!label _label)
          (set `self.combo?` false)
          (`SceneComponent.K2_SetRelativeRotation` _mesh (`KismetMathLibrary.MakeRotator` 0.0 0.0 -90.0) false false))
        (:`OnInterrupted`
          (goto _label))
        (:`OnNotifyBegin`
          (if (and (`self.isattacking`) (`self.combo?`))
            (set `self.combo?` false)
            (else
              (`AnimInstance.Montage_Stop` (`SkeletalMeshComponent.GetAnimInstance` (`Character.Mesh` (`self.PlayerReff`))) 1.0 "/Game/Dank/Player1/animation/YTanimations/Animations/montag/Two_Hand_Sword_Combo_Montage.Two_Hand_Sword_Combo_Montage")))))
      (else
        (set `self.combo?` true)))))

(event `DamageTrace`
  (bind _playerreff (`self.PlayerReff`))
  ; sword traces
  (`KismetSystemLibrary.SphereTraceSingleForObjects` :`Start` (`SceneComponent.K2_GetComponentLocation` (`/Game/ThirdPerson/Blueprints/BP_ThirdPersonCharacter.start_trace` _playerreff)) :`End` (`SceneComponent.K2_GetComponentLocation` (`/Game/ThirdPerson/Blueprints/BP_ThirdPersonCharacter.end_trace` _playerreff)) :`Radius` 10.0 :`ObjectTypes` (`|MakeArray` "ObjectTypeQuery3" :!type "EObjectTypeQuery Enum") :`DrawDebugType` "ForOneFrame"))